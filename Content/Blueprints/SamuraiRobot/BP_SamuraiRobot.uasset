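; BP_SamuraiRobot is a samurai robot character that makes melee attacks, can be knocked upward and plays a hurt montage when damaged.
; PerformAttack plays a double-attack montage, while separate events toggle the attack hitbox's overlaps and visibility.
; Hitbox overlaps damage any other actor, while OnAttack damages overlapping actors passing IsActorEvil, which compares moral alignment to a fixed value.
; It reports a fixed moral alignment and always answers false to CheckIfIsAttacking.
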(event `/Game/Blueprints/Interfaces/BPI_Attacker.PerformAttack`
  (`|PlayMontage` (`self.Mesh`) "/Game/Art/SamuraiRobot/TwoHandWeaponCombo/AM_DoubleAttack.AM_DoubleAttack"))

(event `/Game/Blueprints/Interfaces/BPI_Being.ReceiveKnockup`
  (params (LaunchVelocity :type "Vector Structure"))
  (`self.LaunchCharacter` LaunchVelocity false true))

(event `self.ReceiveAnyDamage`
  (params (Damage :type "Float (single-precision)") (DamageType :type "DamageType Object Reference") (InstigatedBy :type "Controller Object Reference") (DamageCauser :type "Actor Object Reference"))
  (`parent.ReceiveAnyDamage` Damage DamageType InstigatedBy DamageCauser)
  (`|PlayMontage` (`self.Mesh`) "/Game/Art/SamuraiRobot/Hurt/AM_Hurt.AM_Hurt"))

(event `/Game/Blueprints/Interfaces/BPI_Attacker.ActivateHitbox`
  ;[0 0 0] Hitbox activation and deactivation
  (set `PrimitiveComponent.bGenerateOverlapEvents` true (`self.AttackHitbox`))
  (`SceneComponent.SetHiddenInGame` (`self.AttackHitbox`) false false))

(event `/Game/Blueprints/Interfaces/BPI_Attacker.DeactivateHitbox`
  ;[0 0 0] Hitbox activation and deactivation
  (set `PrimitiveComponent.bGenerateOverlapEvents` false (`self.AttackHitbox`))
  (`SceneComponent.SetHiddenInGame` (`self.AttackHitbox`) true false))

(event `self.AttackHitbox.OnComponentBeginOverlap`
  (params (OverlappedComponent :type "PrimitiveComponent Object Reference") (OtherActor :type "Actor Object Reference") (OtherComp :type "PrimitiveComponent Object Reference") (OtherBodyIndex :type Integer) (bFromSweep :type Boolean) (SweepResult :type "HitResult Structure (by ref)"))
  ;[0 0 0] Deal damage when hitbox overlaps an actor
  (if (!= OtherActor self)
    (`GameplayStatics.ApplyDamage` OtherActor 1.0 (`self.GetController`) self)))

(fn `CheckIfIsAttacking`
  (returns (bIsAttacking :type Boolean))
  (return false))

(fn `GetMoralAlignment`
  (returns (Alignment :type "/Game/Blueprints/Enumerations/EMoralAlignment Enum"))
  (return "NewEnumerator2"))

(fn `OnAttack`
  (locals (HitboxOverlappedActors :type "Array of Actor Object Reference") (AttackLaunchVelocity :type "Float (double-precision)" :default 2000.0))
  (bind _output_get (set `local.HitboxOverlappedActors` (`PrimitiveComponent.GetOverlappingActors` (`self.AttackHitbox`) null)))
  (for _array_element _output_get
    (bind _alignment (message `/Game/Blueprints/Interfaces/BPI_Being.GetMoralAlignment` _array_element))
    (if (`|EnumInequality` _alignment "NewEnumerator2")
      (`GameplayStatics.ApplyDamage` _array_element 1.0 null self))))

(fn `UserConstructionScript`
  (`parent.UserConstructionScript`))