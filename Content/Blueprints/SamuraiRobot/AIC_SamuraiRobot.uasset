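; AI controller for the Samurai Robot that runs BT_SamuraiRobot and targets actors of Good moral alignment.
; Perception updates check each actor's alignment, and a new target is cached and written to the Blackboard.
; FaceAttackTarget rotates the pawn toward that target using only X and Y positions.
; Origin and patrol Blackboard locations are placeholders set to zero, with their intended calculations unwired and a TODO to fix them.
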(event `self.ReceiveBeginPlay`
  (`self.RunBehaviorTree` "/Game/Blueprints/SamuraiRobot/BT_SamuraiRobot.BT_SamuraiRobot")
  ;[0.05786 0.0415 0.1562] TODO: Fix patrol and origin location initialization.
  (`self.InitOriginLocation`)
  (`self.InitPatrolLocation` 4000.0))

(event `self.AIPerception.OnTargetPerceptionUpdated`
  (params (Actor :type "Actor Object Reference") (Stimulus :type "AIStimulus Structure"))
  (bind _alignment (message `/Game/Blueprints/Being/BPI_Being.GetMoralAlignment` Actor))
  (switch `/Game/Blueprints/Enumerations/EMoralAlignment` _alignment
    (:`NewEnumerator0`
      (`self.SetAttackTarget` Actor))))

(event `self.FaceAttackTarget`
  (bind _returnvalue (`self.K2_GetPawn`))
  (bind (_returnvalue_x _returnvalue_y) (`KismetMathLibrary.BreakVector` (`self.K2_GetActorLocation` _returnvalue)))
  (bind _attack_target (`self.Attack Target`)
    (:`then`
      (bind (_returnvalue_x_2 _returnvalue_y_2) (`KismetMathLibrary.BreakVector` (`self.K2_GetActorLocation` _attack_target)))
      (`self.K2_SetActorRotation` _returnvalue (`KismetMathLibrary.FindLookAtRotation` (`KismetMathLibrary.MakeVector` _returnvalue_x _returnvalue_y) (`KismetMathLibrary.MakeVector` _returnvalue_x_2 _returnvalue_y_2)) false))
    (:`else`)))

(fn `GetAttackTarget`
  (returns (AttackTarget :type "Actor Object Reference"))
  (return (`self.Attack Target`)))

(fn `InitOriginLocation`
  (`BlackboardComponent.SetValueAsVector` (`self.Blackboard`) "OriginLocation" (`KismetMathLibrary.Vector_Zero`)))

(fn `InitPatrolLocation`
  (params (PatrolDistance :type "Float (double-precision)" :default 1000.0))
  (`BlackboardComponent.SetValueAsVector` (`self.Blackboard`) "PatrolLocation" (`KismetMathLibrary.Vector_Zero`)))

(fn `SetAttackTarget`
  (params (AttackTarget :type "Actor Object Reference"))
  (returns (SameAsBefore :type Boolean))
  (if (!= AttackTarget (`self.Attack Target`))
    (bind _output_get (set `self.Attack Target` AttackTarget))
    (`BlackboardComponent.SetValueAsObject` (`self.Blackboard`) (`self.AttackTargetBlackboardName`) _output_get)
    (return false)
    (else
      (return true))))

(fn `UserConstructionScript`)