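; Samurai robot character Blueprint that supplies attack hitboxes, stun reaction and destruction sound on top of its parent class.
; ActivateHitbox spawns timed BP_Hitbox actors from shape components: the default attack attaches to the robot, while Decapitate stays unattached with its own damage.
; Stuns call the parent and play a hurt montage, and destruction plays a heavy hit sound.
; It reports a fixed moral alignment and never reports itself as attacking.
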(event `/Game/Blueprints/Interfaces/BPI_Attacker.ActivateHitbox`
  (params (HitboxName :type Name) (ActiveDuration :type "Float (single-precision)"))
  (bind _decapitatehitboxshape (`self.DecapitateHitboxShape`))
  (bind _attackhitboxshape (`self.AttackHitboxShape`))
  (switch `name` HitboxName
    (:`Default`
      (bind _returnvalue (`|SpawnActorFromClass` "/Game/Blueprints/Hitbox/BP_Hitbox.BP_Hitbox_C" (`SceneComponent.K2_GetComponentToWorld` _attackhitboxshape) "Undefined" "OverrideRootScale" null ActiveDuration (`BoxComponent.BoxExtent` _attackhitboxshape) self 1.0 null self))
      (`self.K2_AttachToActor` _returnvalue self "None" "KeepWorld" "KeepWorld" "KeepWorld" true))
    (:`DecapitateHitbox`
      (`|SpawnActorFromClass` "/Game/Blueprints/Hitbox/BP_Hitbox.BP_Hitbox_C" (`SceneComponent.K2_GetComponentToWorld` _decapitatehitboxshape) "Undefined" "OverrideRootScale" null ActiveDuration (`BoxComponent.BoxExtent` _decapitatehitboxshape) self (`self.DecapitateDamage`) null self))))

(event `/Game/Blueprints/Being/BP_Being.OnStunned`
  (params (Duration :type "Float (single-precision)"))
  (`parent.OnStunned` Duration)
  (`|PlayMontage` (`self.Mesh`) "/Game/Art/SamuraiRobot/Hurt/AM_Hurt.AM_Hurt"))

(event `self.ReceiveDestroyed`
  (`GameplayStatics.SpawnSoundAtLocation` "/Game/Audio/A_HeavyHitShort.A_HeavyHitShort" (`self.K2_GetActorLocation`) (struct) 2.0 1.5 0.0 null null))

(fn `CheckIfIsAttacking`
  (returns (bIsAttacking :type Boolean))
  (return false))

(fn `GetMoralAlignment`
  (returns (Alignment :type "/Game/Blueprints/Enumerations/EMoralAlignment Enum"))
  (return "NewEnumerator2"))

(fn `UserConstructionScript`
  (`parent.UserConstructionScript`))