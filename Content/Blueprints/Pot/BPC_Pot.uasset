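; BPC_Pot is a damageable ceramic pot that breaks when its health runs out.
; It extends parent damage handling, then plays a damaged sound while health remains, or a breaking sound and destroys itself after a brief delay for emphasis.
; Construction registers its static mesh and default material in the FlashableMeshes arrays.
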(event `self.ReceiveAnyDamage`
  (params (Damage :type "Float (single-precision)") (DamageType :type "DamageType Object Reference") (InstigatedBy :type "Controller Object Reference") (DamageCauser :type "Actor Object Reference"))
  (bind _returnvalue (`self.K2_GetActorLocation`))
  (`parent.ReceiveAnyDamage` Damage DamageType InstigatedBy DamageCauser)
  ;[0 0 0] Damage and Destruction SFX
  (if (<= (`self.HealthPoints`) 0.0)
    (`GameplayStatics.SpawnSoundAtLocation` "/Game/Audio/Ceramic/A_CeramicBreaking_Cue.A_CeramicBreaking_Cue" _returnvalue (struct) 1.0 1.0 0.0 null null)
    (`KismetSystemLibrary.Delay` 0.05) ; A small delay to enphatize its destruction.
    (`self.K2_DestroyActor`)
    (else
      (`GameplayStatics.SpawnSoundAtLocation` "/Game/Audio/Ceramic/A_CeramicDamaged_Cue.A_CeramicDamaged_Cue" _returnvalue (struct) 0.6 1.0 0.0 null null))))

(fn `UserConstructionScript`
  (bind _staticmesh (`self.StaticMesh`))
  (`parent.UserConstructionScript`)
  (`KismetArrayLibrary.Array_Add` (`self.FlashableMeshes`) _staticmesh)
  (`KismetArrayLibrary.Array_Add` (`self.FlashableMeshesDefaultMaterials`) (`PrimitiveComponent.GetMaterial` _staticmesh 0)))