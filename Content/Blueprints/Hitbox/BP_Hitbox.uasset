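; BP_Hitbox is a short-lived actor that damages actors overlapping its box on behalf of an AttackOwner, then destroys itself after Lifespan.
; Each tick it runs a debug-drawn multi box trace in place, optionally skipping actors of the owner's class.
; ApplyDamageOnce uses AddUnique on the trace ignore list, seeded with the owner, so each victim is damaged once.
; Successful hits credit the owner and fire OnDamageApplied.
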(event `self.ReceiveBeginPlay`
  (`KismetArrayLibrary.Array_AddUnique` (`self.TraceIgnoredActors`) (`self.AttackOwner`))
  (`KismetSystemLibrary.K2_SetTimerDelegate` (delegate `Event Lifespan End`) (`self.Lifespan`)))

(event `Event Lifespan End`
  (`self.K2_DestroyActor`))

(event `self.ReceiveTick`
  (params (DeltaSeconds :type "Float (single-precision)"))
  (bind _returnvalue (`self.K2_GetActorLocation`))
  (bind _outhits (`KismetSystemLibrary.BoxTraceMulti` _returnvalue _returnvalue (`self.BoxExtent`) (`self.K2_GetActorRotation`) "TraceTypeQuery3" false (`self.TraceIgnoredActors`) "ForOneFrame"))
  (for _array_element _outhits
    (bind (_bblockinghit _binitialoverlap _time _distance _location _impactpoint _normal _impactnormal _physmat _hitactor) (`GameplayStatics.BreakHitResult` _array_element))
    (if (or (!= (`GameplayStatics.GetObjectClass` _hitactor) (`GameplayStatics.GetObjectClass` (`self.AttackOwner`))) (`self.bCanHitActorsOfTheSameClassAsOwner`))
      (`self.Apply Damage Once` _hitactor (`self.BaseDamage`) (`self.Damage Type Class`)))))

(fn `Apply Damage Once`
  (params (`Damaged Actor` :type "Actor Object Reference (by ref)") (BaseDamage :type "Float (double-precision)" :default 1.0) (DamageTypeClass :type "DamageType Class Reference"))
  (bind _attackowner (`self.AttackOwner`))
  (if (`KismetSystemLibrary.IsValid` `Damaged Actor`)
    (bind _returnvalue (`KismetArrayLibrary.Array_AddUnique` (`self.TraceIgnoredActors`) `Damaged Actor`))
    (if (!= _returnvalue (`self.INDEX_NONE`))
      (`GameplayStatics.ApplyDamage` `Damaged Actor` BaseDamage (`self.GetInstigatorController` _attackowner) _attackowner DamageTypeClass)
      (`self.OnDamageApplied` `Damaged Actor`))))

(fn `UserConstructionScript`
  (locals (cBoxExtent :type "Vector Structure") (cLifespan :type "Float (double-precision)")))