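; BP_GameState is a game state hub for enemy-death notifications, selective time stops and global hitstop.
; Registered listeners receive enemy-destroyed messages, while registered actors have their CustomTimeDilation set to zero or one to stop and resume time.
; Both broadcasts prune invalid entries through a sanitized array.
; Hitstop lowers global time dilation and sets a timer, scaling its duration by that dilation to compensate for slowed time.
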(event `/Game/Blueprints/GameState/BPI_GameState.AlertEnemyDestroyed`
  (params (EnemyDestroyed :type "Actor Object Reference"))
  (`self.BroadcastEnemyDestroyed`))

(event `/Game/Blueprints/GameState/BPI_GameState.AddEnemyDestroyedListener`
  (params (ListenerToAdd :type "Object Object Reference"))
  (`KismetArrayLibrary.Array_AddUnique` (`self.EnemyDestroyedListeners`) ListenerToAdd))

(event `/Game/Blueprints/GameState/BPI_GameState.Hitstop`
  (params (Duration :type "Float (single-precision)"))
  (`self.StartHitstop` Duration))

(event `/Game/Blueprints/GameState/BPI_GameState.AddTimeStoppableActor`
  (params (ActorToAdd :type "Actor Object Reference"))
  (`KismetArrayLibrary.Array_AddUnique` (`self.TimeStoppableActors`) ActorToAdd))

(event `/Game/Blueprints/GameState/BPI_GameState.ResumeTime`
  (`self.SetTimeDilationOnActors` 1.0))

(event `/Game/Blueprints/GameState/BPI_GameState.StopTime`
  (`self.SetTimeDilationOnActors` 0.0))

(event `EventEndHitstop`
  (`GameplayStatics.SetGlobalTimeDilation` 1.0))

(fn `BroadcastEnemyDestroyed`
  (locals (SanitizedEnemyDestroyedListenersArray :type "Array of Object Object Reference"))
  (set `local.SanitizedEnemyDestroyedListenersArray` (`self.EnemyDestroyedListeners`))
  (for _array_element (`self.EnemyDestroyedListeners`)
    (if (`KismetSystemLibrary.IsValid` _array_element)
      (message `/Game/Blueprints/GameState/BPI_EnemyDestroyedListener.OnAnyEnemyDestroyed` _array_element)
      (else
        (`KismetArrayLibrary.Array_RemoveItem` (`local.SanitizedEnemyDestroyedListenersArray`) _array_element))))
  (set `self.EnemyDestroyedListeners` (`local.SanitizedEnemyDestroyedListenersArray`)))

(fn `SetTimeDilationOnActors`
  (params (TimeDilation :type "Float (double-precision)"))
  (locals (SanitizedArray :type "Array of Actor Object Reference"))
  (set `local.SanitizedArray` (`self.TimeStoppableActors`))
  (for _array_element (`self.TimeStoppableActors`)
    (if (`KismetSystemLibrary.IsValid` _array_element)
      (set `Actor.CustomTimeDilation` TimeDilation _array_element)
      (else
        (`KismetArrayLibrary.Array_RemoveItem` (`local.SanitizedArray`) _array_element))))
  (set `self.TimeStoppableActors` (`local.SanitizedArray`)))

(fn `StartHitstop`
  (params (Duration :type "Float (double-precision)" :default 0.1))
  (locals (TimeStopTimeDilation :type "Float (double-precision)" :default 0.0001))
  (bind _timestoptimedilation (`local.TimeStopTimeDilation`))
  (`GameplayStatics.SetGlobalTimeDilation` _timestoptimedilation)
  (`KismetSystemLibrary.K2_SetTimerDelegate` (`|CreateDelegate` :!event `EventEndHitstop`) (* Duration _timestoptimedilation)))

(fn `UserConstructionScript`)