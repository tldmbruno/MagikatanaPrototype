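; BP_GameMode is a single-player game mode that respawns the player after their pawn is destroyed.
; It caches the controller on login, binds to each restarted pawn's OnDestroyed, and calls RestartPlayer again after a short delay.
; An overridden FindPlayerStart returns a stored start actor set through UpdateSpawnLocationActor, acting as a movable respawn point, and otherwise falls back to a PlayerStart in the level.
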(event `self.K2_PostLogin`
  (params (NewPlayer :type "PlayerController Object Reference"))
  (bind _output_get (set `self.PlayerControllerReference` NewPlayer)) ; Since this is a singleplayer game,\nwe can store this reference for later.
  (`self.RestartPlayer` _output_get))

(event `self.K2_OnRestartPlayer`
  (params (NewPlayer :type "Controller Object Reference"))
  (add `self.OnDestroyed` (`Controller.K2_GetPawn` NewPlayer) (delegate `Player_OnDestroyed`)))

(event `Player_OnDestroyed` :!signature `self.OnDestroyed`
  (params (DestroyedActor :type "Actor Object Reference"))
  (`KismetSystemLibrary.Delay` 1.0)
  (`self.RestartPlayer` (`self.PlayerControllerReference`)))

(event `/Game/Blueprints/Interfaces/BPI_SpawnLocationUpdater.UpdateSpawnLocationActor`
  (params (NewStartActor :type "Actor Object Reference"))
  (set `self.PlayerStartActor` NewStartActor))

(fn `FindPlayerStart`
  (params (Player :type "Controller Object Reference") (IncomingName :type String))
  (returns (ReturnValue :type "Actor Object Reference"))
  (bind _playerstartactor (`self.PlayerStartActor`)
    (:`then`
      (return _playerstartactor))
    (:`else`
      (bind _returnvalue (`GameplayStatics.GetActorOfClass` "/Script/Engine.PlayerStart"))
      (return _returnvalue))))

(fn `UserConstructionScript`)