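; Trigger actor that fires its listeners once a target number of enemies has been destroyed while it is active.
; It registers with the GameState for enemy-destroyed messages, and incoming trigger activation and deactivation events switch counting on and off.
; On reaching the target it resets the count, sends activation to every TriggerListener, and destroys itself unless it is retriggerable.
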(event `/Game/Blueprints/Interfaces/BPI_TriggerListener.OnTriggerActivation`
  (params (TriggerActor :type "Actor Object Reference") (TriggerCauser :type "Actor Object Reference"))
  (set `self.bIsCountingKills` true))

(event `/Game/Blueprints/Interfaces/BPI_TriggerListener.OnTriggerDeactivation`
  (params (TriggerActor :type "Actor Object Reference") (TriggerCauser :type "Actor Object Reference"))
  (set `self.bIsCountingKills` false))

(event `self.ReceiveBeginPlay`
  (message `/Game/Blueprints/GameState/BPI_GameState.AddEnemyDestroyedListener` (`GameplayStatics.GetGameState`) self))

(event `/Game/Blueprints/GameState/BPI_EnemyDestroyedListener.OnAnyEnemyDestroyed`
  (if (`self.bIsCountingKills`)
    (bind _result (`/Engine/EditorBlueprintResources/StandardMacros.IncrementInt` (`self.KillsSinceActivation`))
      (:`  `
        (if (>= _result (`self.KillTargetCount`))
          (`self.OnKillTargetAchieved` null)
          (set `self.KillsSinceActivation` 0))))))

(event `OnKillTargetAchieved`
  (params (KillerOfTheLastOne :type "Actor Object Reference"))
  (for _array_element (`self.TriggerListeners`)
    (message `/Game/Blueprints/Interfaces/BPI_TriggerListener.OnTriggerActivation` _array_element self KillerOfTheLastOne))
  (if (not (`self.bIsRetriggerable`))
    (`self.K2_DestroyActor`)))

(fn `UserConstructionScript`)