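; BP_CombatBarrier is a toggleable barrier actor, named for combat encounters, that switches between blocking and absent.
; It starts hidden with collision disabled on BeginPlay.
; Each OnTriggerActivation event alternates through a FlipFlop between showing it with collision and hiding it without.
; When it hides on the second activation, it destroys itself unless CanReappear is set.
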(event `self.ReceiveBeginPlay`
  (`self.HideActor`))

(event `/Game/Blueprints/Interfaces/BPI_TriggerListener.OnTriggerActivation`
  (params (TriggerActor :type "Actor Object Reference") (TriggerCauser :type "Actor Object Reference"))
  (`/Engine/EditorBlueprintResources/StandardMacros.FlipFlop`
    (:`A`
      (`self.ShowActor`))
    (:`B`
      (`self.HideActor`)
      (if (not (`self.bCanReappear`))
        (`self.K2_DestroyActor`)))))

(fn `HideActor`
  (`self.SetActorHiddenInGame` true)
  (`self.SetActorEnableCollision` false))

(fn `ShowActor`
  (`self.SetActorHiddenInGame` false)
  (`self.SetActorEnableCollision` true))

(fn `UserConstructionScript`)