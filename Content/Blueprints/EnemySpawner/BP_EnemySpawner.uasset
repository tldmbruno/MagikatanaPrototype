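; Enemy spawner actor that spawns a configurable enemy class at its own transform when it receives a trigger activation.
; A short random delay precedes each spawn, which plays a sound and uses interface messages to apply an optional starting health override.
; Blind enemies have their AI controller unpossessed, while others can be forced to attack the player immediately.
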(event `/Game/Blueprints/Interfaces/BPI_TriggerListener.OnTriggerActivation`
  (params (TriggerActor :type "Actor Object Reference") (TriggerCauser :type "Actor Object Reference"))
  (`KismetSystemLibrary.Delay` (`KismetMathLibrary.RandomFloatInRange` 0.0 0.5))
  (`self.Spawn Enemy`))

(fn `Spawn Enemy`
  (bind _enemystartinghealthpoints (`self.EnemyStartingHealthPoints`))
  (bind _returnvalue (`|SpawnActorFromClass` (`self.EnemyClass`) (`self.GetTransform`) "AdjustIfPossibleButAlwaysSpawn" "OverrideRootScale" null false null))
  (if (not (== _enemystartinghealthpoints -1.0))
    (message `/Game/Blueprints/Being/BPI_Being.SetHealthPointsPurely` _returnvalue _enemystartinghealthpoints))
  (`GameplayStatics.PlaySoundAtLocation` "/Game/Audio/A_MarkApplied.A_MarkApplied" (`self.K2_GetActorLocation`) (struct) 0.4 3.0 0.5 null null null)
  (if (not (`self.bEnemyIsBlind`))
    (if (`self.bSpawnAlreadyAggroed`)
      (message `/Game/Blueprints/Enemy/BPI_Enemy.ForceAttackTargetOnActor` _returnvalue (`GameplayStatics.GetPlayerPawn` 0)))
    (else
      (`Controller.UnPossess` (`AIBlueprintHelperLibrary.GetAIController` _returnvalue))
      (return))))

(fn `UserConstructionScript`)