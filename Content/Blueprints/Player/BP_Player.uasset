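; First-person player character with melee attacks, an energy-limited dash, wall jumps and a timed enemy-marking combo.
; Movement input selects a forward slash or a launching uppercut, and hits restore dash energy.
; Dashes pass through pawns, then box-trace the path to mark beings of other alignments.
; A timeline drives mark charge: activating at full charge detonates marked enemies with brief slow motion, while mistiming or expiry clears them.
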(event `self.ReceiveBeginPlay`
  ;[0 0 0] Add HUD to Viewport
  (bind _returnvalue (`|CreateWidget` "/Game/Blueprints/UI/WBP_PlayerHUD.WBP_PlayerHUD_C"))
  (bind _output_get (set `self.PlayerHUD` _returnvalue))
  (`UserWidget.AddToViewport` _output_get 0))

(event `InputAction|Jump`
  (params (Key :type "Key Structure"))
  ;[0 0 0] Jumping & Landing
  (:`Pressed`
    (bind _bdidwalljump_ (`self.TryWallJump`))
    (if (not _bdidwalljump_)
      (`self.Jump`)))
  (:`Released`
    (`self.StopJumping`)))

(event `self.K2_OnMovementModeChanged`
  (params (PrevMovementMode :type "EMovementMode Enum" :default "MOVE_None") (NewMovementMode :type "EMovementMode Enum" :default "MOVE_None") (PrevCustomMode :type Byte) (NewCustomMode :type Byte))
  ;[0 0 0] Jumping & Landing
  (`self.ResetWallJumpsCountIfOnGround`))

(event `InputAction|Attack`
  (params (Key :type "Key Structure"))
  ;[0 0 0] Attack Action
  (:`Pressed`
    (switch `/Game/Blueprints/Enumerations/EInputDirections` (`self.GetInputDirectionEnum`)
      (:`NewEnumerator0`
        (`self.SlashForward` :!label _label)
        (bind _decalworldlocation (`self.FindCrosshairDecalLocation`))
        (`GameplayStatics.SpawnDecalAtLocation` "/Game/StarterContent/Materials/M_Metal_Gold.M_Metal_Gold" (10.0 10.0 10.0) _decalworldlocation (struct :`Pitch` -90.0) 10.0))
      (:`NewEnumerator1`
        (goto _label))
      (:`NewEnumerator4`
        (`self.Uppercut`)
        (`KismetSystemLibrary.PrintString` "UPPERCUT!")))))

(event `InputAction|Dash`
  (params (Key :type "Key Structure"))
  ;[0 0 0] Dash
  (:`Pressed`
    (`PrimitiveComponent.SetCollisionResponseToChannel` (`self.CapsuleComponent`) "ECC_Pawn" "ECR_Ignore")
    (`PrimitiveComponent.SetCollisionResponseToChannel` (`self.Mesh`) "ECC_Pawn" "ECR_Ignore")
    (`self.Dash Towards Velocity`)))

(event `Event OnDashEnd`
  ;[0 0 0] Dash
  (set `self.bIsDashing?` false)
  (`PrimitiveComponent.SetCollisionResponseToChannel` (`self.CapsuleComponent`) "ECC_Pawn" "ECR_Block")
  (`PrimitiveComponent.SetCollisionResponseToChannel` (`self.Mesh`) "ECC_Pawn" "ECR_Block")
  (set `self.LastDashEndLocation` (`self.K2_GetActorLocation`))
  (bind _markedenemies (`self.Get Dashed Through Enemies`))
  (`KismetArrayLibrary.Array_Append` (`self.MarkedEnemies`) _markedenemies)
  (if (> (`KismetArrayLibrary.Array_Length` _markedenemies) 0)
    (`self.Event OnMarkApplied`)))

(event `Event OnMarkApplied`
  ;[0 0 0] Marking
  (bind (_direction _markcharge) (`Timeline|MarkProgressTimeline` :!via `PlayFromStart` :!label _label_2)
    (:`Update`
      (set `self.MarkCharge` _markcharge))
    (:`Finished`
      (`self.Event OnMarkDepleted`))))

(event `Event OnMarkSuccessfullyActivated`
  ;[0 0 0] Marking
  (`|ExecutionSequence`
    (:`then_0`
      (goto _label_2 :!via `Stop`))
    (:`then_1`
      (set `self.MarkCharge` 0.0)
      (`self.Damage Beings` (`self.MarkedEnemies`) (`self.MarkActivationDamage`) "/Game/StarterContent/Particles/P_Explosion.P_Explosion")
      (`KismetArrayLibrary.Array_Clear` (`self.MarkedEnemies`))
      (`GameplayStatics.SetGlobalTimeDilation` 0.1)
      (`KismetSystemLibrary.Delay` 0.1)
      (`GameplayStatics.SetGlobalTimeDilation` 1.0))))

(event `Event OnMarkDepleted`
  ;[0 0 0] Marking
  (`KismetArrayLibrary.Array_Clear` (`self.MarkedEnemies`)))

(event `InputAction|ActivateMark`
  (params (Key :type "Key Structure"))
  ;[0 0 0] Marking
  (:`Pressed`
    (if (>= (`self.MarkCharge`) 1.0)
      (`KismetSystemLibrary.PrintString` "ACTIVATED")
      (`self.Event OnMarkSuccessfullyActivated`)
      (else
        (`KismetSystemLibrary.PrintString` "FAIL")
        (`self.Event OnMarkDepleted`)))))

(fn `Damage Beings`
  (params (Beings :type "Array of /Game/Blueprints/Being/BP_Being Object Reference") (Damage :type "Float (double-precision)") (Particles :type "ParticleSystem Object Reference"))
  (locals (LocalMarkedEnemies :type "Array of /Game/Blueprints/Interfaces/BPI_Being Interface") (DamageMultiplier :type "Float (double-precision)" :default 3.0))
  (for _array_element Beings
    (`/Engine/EditorBlueprintResources/StandardMacros.IsValid` _array_element
      (:`Is Valid`
        (`GameplayStatics.SpawnEmitterAtLocation` (`local.Particles`) (`self.K2_GetActorLocation` _array_element) (struct) (3.0 3.0 3.0))
        (`GameplayStatics.ApplyDamage` _array_element (`local.Damage`))))))

(fn `Dash Towards Velocity`
  (locals (DashDirection :type "Vector Structure" :default (0.0 0.0 0.0)) (DashStrength :type "Float (double-precision)" :default 20000.0) (IsStandingStill :type Boolean :default false))
  (bind (_dashdirection_x _dashdirection_y) (`KismetMathLibrary.BreakVector` (`local.DashDirection`)))
  (bind (_start _end) (`self.GetWorldInputDirection` (`local.DashStrength`)))
  (if (> (`self.DashEnergy`) 0.0)
    (`/Engine/EditorBlueprintResources/StandardMacros.DecrementFloat` (`self.DashEnergy`)
      (:`  `
        (set `self.LastDashStartingLocation` (`self.K2_GetActorLocation`))
        (bind _output_get (set `local.DashDirection` (- _end _start)))
        (set `local.IsStandingStill` (== _output_get (`KismetMathLibrary.Vector_Zero`)))
        (`|ExecutionSequence`
          (:`then_0`
            (if (`local.IsStandingStill`)
              (set `local.DashDirection` (* (`self.GetActorForwardVector`) (`local.DashStrength`)))))
          (:`then_1`
            (`CharacterMovementComponent.AddImpulse` (`self.CharacterMovement`) (`KismetMathLibrary.MakeVector` _dashdirection_x _dashdirection_y 100.0) true)
            (set `self.bIsDashing?` true)
            (`KismetSystemLibrary.K2_SetTimerDelegate` (`|CreateDelegate` :!event `Event OnDashEnd`) 0.2)))))
    (else
      (`KismetSystemLibrary.PrintString` "Not enough DashEnergy"))))

(fn `FindCrosshairDecalLocation`
  (returns (DecalWorldLocation :type "Vector Structure"))
  (locals (OverlappingActorsWithoutPlayer :type "Array of Actor Object Reference"))
  (bind _firstpersoncamera (`self.FirstPersonCamera`))
  (bind _returnvalue (`SceneComponent.K2_GetComponentLocation` _firstpersoncamera))
  (bind _outhit (`KismetSystemLibrary.LineTraceSingle` _returnvalue (+ _returnvalue (* (`SceneComponent.GetForwardVector` _firstpersoncamera) 700.0)) "TraceTypeQuery1" true))
  (return (`.Location` (`GameplayStatics.BreakHitResult` _outhit))))

(fn `Get Dashed Through Enemies`
  (returns (MarkedEnemies :type "Array of /Game/Blueprints/Being/BP_Being Object Reference"))
  (locals (ActorsInDashTrajectory :type "Array of Actor Object Reference") (MarkedActors :type "Array of HitResult Structure") (MarkedBeings :type "Array of /Game/Blueprints/Being/BP_Being Object Reference"))
  (bind _outhits (`KismetSystemLibrary.BoxTraceMulti` :`Start` (`self.LastDashStartingLocation`) :`End` (`self.LastDashEndLocation`) :`HalfSize` (`BoxComponent.BoxExtent` (`self.DashSlashHitbox`)) :`Orientation` (`self.K2_GetActorRotation`) :`TraceChannel` "TraceTypeQuery3" :`DrawDebugType` "ForDuration" :`TraceColor` (struct :`R` 1.0 :`G` 0.101385 :`B` 0.930939 :`A` 1.0) :`TraceHitColor` (struct :`R` 0.376913 :`G` 0.603187 :`B` 1.0 :`A` 1.0)))
  (bind _output_get (set `local.MarkedActors` _outhits))
  (for _array_element _output_get
    (bind _being (message `/Game/Blueprints/Interfaces/BPI_Being.GetBeing` (`.HitActor` (`GameplayStatics.BreakHitResult` _array_element))))
    (bind _alignment (message `/Game/Blueprints/Interfaces/BPI_Being.GetMoralAlignment` _being))
    (if (`|EnumInequality` _alignment "NewEnumerator0")
      (`KismetArrayLibrary.Array_AddUnique` (`local.MarkedBeings`) _being)))
  (return (`local.MarkedBeings`)))

(fn `GetInputDirectionEnum`
  (returns (Enum :type "/Game/Blueprints/Enumerations/EInputDirections Enum"))
  (locals (bIsStandingStill :type Boolean) (RelativeInputVectorNormalized :type "Vector2D Structure") (bIsForwardZero :type Boolean) (bIsRightZero :type Boolean))
  (bind _relativeinputvectornormalized_x (`KismetMathLibrary.BreakVector2D` (`local.RelativeInputVectorNormalized`)))
  (bind (_relativeinputvectornormalized_x_2 _relativeinputvectornormalized_y) (`KismetMathLibrary.BreakVector2D` (`local.RelativeInputVectorNormalized`)))
  (bind _output_get (set `local.RelativeInputVectorNormalized` (`KismetMathLibrary.MakeVector2D` (`self.GetInputAxisValue`) (`self.GetInputAxisValue`))))
  (set `local.bIsForwardZero` (== (`KismetMathLibrary.BreakVector2D` _output_get) 0.0))
  (set `local.bIsRightZero` (== (`.Y` (`KismetMathLibrary.BreakVector2D` _output_get)) 0.0))
  (if (`local.bIsForwardZero`)
    (if (`local.bIsRightZero`)
      (return "NewEnumerator0")
      (else
        (return (select `bool` (> _relativeinputvectornormalized_y 0.0) :`false` "NewEnumerator2" :`true` "NewEnumerator3" :!type "/Game/Blueprints/Enumerations/EInputDirections Enum"))))
    (else
      (return (select `bool` (> _relativeinputvectornormalized_x 0.0) :`false` "NewEnumerator4" :`true` "NewEnumerator1" :!type "/Game/Blueprints/Enumerations/EInputDirections Enum")))))

(fn `GetMoralAlignment`
  (returns (Alignment :type "/Game/Blueprints/Enumerations/EMoralAlignment Enum"))
  (return "NewEnumerator0"))

(fn `GetWorldInputDirection`
  (params (DistanceFromStartToEnd :type "Float (double-precision)"))
  (returns (Start :type "Vector Structure") (End :type "Vector Structure"))
  (locals (TraceEndLocation :type "Vector Structure"))
  (bind _returnvalue (`self.K2_GetActorLocation`))
  (return _returnvalue (+ (* (`self.GetActorRightVector`) (* (`self.GetInputAxisValue`) DistanceFromStartToEnd)) _returnvalue (* (`self.GetActorForwardVector`) (* (`self.GetInputAxisValue`) DistanceFromStartToEnd)))))

(fn `Recover One Point Of Dash Energy`
  (bind _dashenergy (`self.DashEnergy`))
  (bind _maximumdashenergy (`self.MaximumDashEnergy`))
  (`/Engine/EditorBlueprintResources/StandardMacros.IncrementFloat` _dashenergy
    (:`  `
      (if (> _dashenergy _maximumdashenergy)
        (set `self.DashEnergy` _maximumdashenergy)))))

(fn `ResetWallJumpsCountIfOnGround`
  (if (`|EnumEquality` (`CharacterMovementComponent.MovementMode` (`self.CharacterMovement`)) "MOVE_Walking")
    (set `self.WallJumpsCount` 0)))

(fn `SlashForward`
  (returns (AmountOfDamagedActors :type Integer))
  (locals (damagedActorsCount :type Integer) (overlappingActorsArray :type Integer) (actorsInSlashHitbox :type "Array of Actor Object Reference") (AttackForwardImpulse :type "Float (double-precision)" :default 500.0))
  (bind (_returnvalue_x _returnvalue_y _returnvalue_z) (`KismetMathLibrary.BreakVector` (* (`self.GetActorForwardVector`) (`local.AttackForwardImpulse`))))
  (bind _output_get (set `local.actorsInSlashHitbox` (`PrimitiveComponent.GetOverlappingActors` (`self.SlashHitbox`) null))) ; Since we are dealing with damage,\nsome actors will destroy themselves.\nStoring them in a local variable prevents\nthe premature exit of the For Each Loop
  (for _array_element _output_get
    (if (!= _array_element (`ActorComponent.GetOwner` (`self.CapsuleComponent`)))
      (`GameplayStatics.ApplyDamage` _array_element (`self.AttackDamage`) (`GameplayStatics.GetPlayerController` 0) (`ActorComponent.GetOwner` (`self.SlashHitbox`)) "/Script/Engine.DamageType")
      (`/Engine/EditorBlueprintResources/StandardMacros.IncrementInt` (`local.damagedActorsCount`)
        (:`  `
          (`/Engine/EditorBlueprintResources/StandardMacros.DoOnce` false
            (:`Completed`
              (`self.Recover One Point Of Dash Energy`)))))))
  (`CharacterMovementComponent.AddImpulse` (`self.CharacterMovement`) (`KismetMathLibrary.MakeVector` _returnvalue_x _returnvalue_y _returnvalue_z) true)
  ;[0.5573 0 0.1356] PLACEHOLDER Animation
  (`SkeletalMeshComponent.PlayAnimation` (`self.Arms`) "/Game/Art/Player/AS_Attack.AS_Attack" false)
  (return (`local.damagedActorsCount`)))

(fn `TryWallJump`
  (returns (`bDidWallJump?` :type Boolean))
  (locals (RelativeWallImpulse :type "Vector Structure") (WallJumpPushBackImpulse :type "Float (double-precision)" :default 2000.0))
  (bind (_start _end) (`self.GetWorldInputDirection` 100.0))
  (bind (_returnvalue_x _returnvalue_y) (`KismetMathLibrary.BreakVector` (`self.GetVelocity`)))
  (if (and (`|EnumEquality` (`CharacterMovementComponent.MovementMode` (`self.CharacterMovement`)) "MOVE_Falling") (< (`self.WallJumpsCount`) (`self.WallJumpsMax`)))
    (bind (_outhit _returnvalue) (`KismetSystemLibrary.LineTraceSingle` _start _end "TraceTypeQuery1"))
    (if _returnvalue
      (bind _output_get (set `local.RelativeWallImpulse` (* (`KismetMathLibrary.Normal` (- _start _end)) (`local.WallJumpPushBackImpulse`))))
      (set `MovementComponent.Velocity` (`KismetMathLibrary.MakeVector` _returnvalue_x _returnvalue_y) (`self.CharacterMovement`))
      (`CharacterMovementComponent.AddImpulse` (`self.CharacterMovement`) (+ _output_get (`KismetMathLibrary.MakeVector` 0.0 0.0 (* (`CharacterMovementComponent.JumpZVelocity` (`self.CharacterMovement`)) 2.0))) true)
      (`/Engine/EditorBlueprintResources/StandardMacros.IncrementInt` (`self.WallJumpsCount`)
        (:`  `
          (return true)))
      (else
        (return false)))
    (else
      (return false))))

(fn `Uppercut`
  (locals (LaunchUpwardsVelocity :type "Vector Structure" :default (0.0 0.0 1000.0)))
  (for _array_element (`PrimitiveComponent.GetOverlappingActors` (`self.SlashHitbox`) null)
    (if (!= _array_element self)
      (bind _being (message `/Game/Blueprints/Interfaces/BPI_Being.GetBeing` _array_element))
      (`self.LaunchCharacter` _being (`local.LaunchUpwardsVelocity`) false true)
      (`GameplayStatics.ApplyDamage` _being (`self.AttackDamage`))
      (`/Engine/EditorBlueprintResources/StandardMacros.DoOnce` false
        (:`Completed`
          (`self.Recover One Point Of Dash Energy`))))))

(fn `UserConstructionScript`)