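; BP_Enemy is a target dummy enemy with a health bar that can be damaged, knocked up and destroyed.
; Any damage lowers its health, fires the OnHealthChanged dispatcher, spawns an explosion and destroys the actor at zero health.
; The dispatcher drives the widget component's progress bar as a fraction of max health.
; Knockup turns on capsule physics, applies a velocity-change impulse and deals damage.
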(event Custom|OnHealthChanged_Event
  (params (PreviousValue :type Float%20%28single-precision%29) (NewValue :type Float%20%28single-precision%29))
  (CallFunction|UpdateHealthBar NewValue))

(event EventBeginPlay
  (CallFunction|InitializeHealthBar)
  (EventDispatchers|BindEventtoOnHealthChanged (delegate Custom|OnHealthChanged_Event)))

(event Game|Damage|EventAnyDamage
  (params (Damage :type Float%20%28single-precision%29) (DamageType :type Damage%20Type%20Object%20Reference) (InstigatedBy :type Controller%20Object%20Reference) (DamageCauser :type Actor%20Object%20Reference))
  (bind _output_get (Variables|Default|SetHealthPoints (|({5333D43C-485C-B500-A330-628C2FF6F612}-Damage) Damage)))
  (Default|CallOnHealthChanged 0.0 _output_get)
  (Effects|SpawnEmitteratLocation "/Game/StarterContent/Particles/P_Explosion.P_Explosion" (Transformation|GetActorLocation))
  (if (<= (Variables|Default|GetHealthPoints) 0.0)
    (Actor|DestroyActor)))

(fn ConstructionScript)

(fn InitializeHealthBar
  (bind _aswbp_health_bar (Utilities|Casting|CastToWBP_HealthBar (UserInterface|GetWidget (Variables|Default|GetHealthBar))))
  (Variables|Default|SetHealthProgressBar (Variables|/Game/Blueprints/TargetDummy/WBP_HealthBar.WBP_HealthBar_C|GetProgressBar_0 _aswbp_health_bar)))

(fn UpdateHealthBar
  (params (NewValue :type Float%20%28single-precision%29))
  (Progress|SetPercent (Variables|Default|GetHealthProgressBar) (|(NewValue/{00F550BA-4E7C-3AD3-89A6-85B64E5D6802}) NewValue)))

(fn GetMainStageComponent
  (return 0))

(fn Knockup
  (params (NewVelocity :type Vector :default "0, 0, 0") (Damage :type Float%20%28single-precision%29))
  (Physics|SetSimulatePhysics (Variables|Default|GetCapsuleComponent) true)
  (Physics|AddImpulse (Variables|Default|GetCapsuleComponent) NewVelocity "None" true)
  (Game|Damage|ApplyDamage 0 Damage 0 0)
  (return true))