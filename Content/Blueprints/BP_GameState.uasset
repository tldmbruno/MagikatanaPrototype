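; BP_GameState tracks enemy kills per round and starts a new round once they reach the spawned count.
; OnEnemyDestroyed increments the destroyed count, broadcasts the change and compares it to the spawned count.
; When the round is cleared, a DoOnce-guarded delay resets both counters, fires OnRoundBegin and re-arms the guard.
; GetEnemyDestroyedCount is a stub that always returns zero.
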(event `/Game/Blueprints/Interfaces/BPI_EnemyDestroyedListener.OnEnemyDestroyed`
  (params (DestroyedActorClass :type "Object Class Reference"))
  (bind _result (`/Engine/EditorBlueprintResources/StandardMacros.IncrementInt` (`self.CurrentRoundEnemyDestroyedCount`))
    (:`  `
      (`self.OnEnemyDestroyedCountChange` _result)
      (if (>= (`self.CurrentRoundEnemyDestroyedCount`) (`self.CurrentRoundEnemySpawnedCount`))
        (`/Engine/EditorBlueprintResources/StandardMacros.DoOnce` false :!label _label
          (:`Completed`
            (`KismetSystemLibrary.PrintString` "NEW ROUND" true true (struct :`R` 1.0 :`G` 0.766463 :`B` 0.093989 :`A` 1.0))
            (`KismetSystemLibrary.Delay` 2.0)
            (set `self.CurrentRoundEnemySpawnedCount` 0)
            (set `self.CurrentRoundEnemyDestroyedCount` 0)
            (`self.OnRoundBegin`)
            (goto _label :!via `Reset`)))))))

(fn `GetEnemyDestroyedCount`
  (returns (Count :type Integer))
  (return 0))

(fn `UserConstructionScript`)