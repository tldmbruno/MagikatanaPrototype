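; Samurai robot character Blueprint that performs a lunging melee attack and reports a fixed moral alignment.
; The Attack event damages actors overlapping AttackHitbox that pass the IsActorEvil check, then launches the robot along its forward vector, overriding vertical velocity.
; IsActorEvil queries each target's alignment by interface message and passes any that differs from the value this robot's GetMoralAlignment returns.
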(event `/Game/Blueprints/Enemy/BPI_MeleeAttacker.Attack`
  (`self.OnAttack`))

(fn `GetMoralAlignment`
  (returns (Alignment :type "/Game/Blueprints/Enumerations/EMoralAlignment Enum"))
  (return "NewEnumerator2"))

(fn `OnAttack`
  (locals (HitboxOverlappedActors :type "Array of Actor Object Reference") (AttackLaunchVelocity :type "Float (double-precision)" :default 2000.0))
  (bind _output_get (set `local.HitboxOverlappedActors` (`PrimitiveComponent.GetOverlappingActors` (`self.AttackHitbox`) null)))
  (for _array_element _output_get
    (bind _alignment (message `/Game/Blueprints/Interfaces/BPI_Being.GetMoralAlignment` _array_element))
    (if (`|EnumInequality` _alignment "NewEnumerator2")
      (`GameplayStatics.ApplyDamage` _array_element 1.0 null self)))
  (`self.LaunchCharacter` (* (`self.GetActorForwardVector`) (`local.AttackLaunchVelocity`)) false true))

(fn `UserConstructionScript`
  (`parent.UserConstructionScript`))