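; Health bar actor for enemies, shown only while a being is near.
; On BeginPlay it links its WBP_HealthBar widget to the parent BP_Enemy, so it expects to be a child actor of one, and initializes the bar.
; VisibilityRange overlaps with BPI_Being actors toggle the root's hidden state, propagated to children.
; Any such actor leaving hides the bar, with no check for others still in range.
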(event `self.ReceiveBeginPlay`
  (if (not (`PrimitiveComponent.IsOverlappingActor` (`self.VisibilityRange`) null))
    (`self.Hide`))
  (bind _aswbp_health_bar (cast `/Game/Blueprints/Enemy/WBP_HealthBar` (`WidgetComponent.GetWidget` (`self.HealthBarWidget`))))
  (bind _asbp_enemy (cast `/Game/Blueprints/Enemy/BP_Enemy` (`self.GetParentActor`)))
  (set `/Game/Blueprints/Enemy/WBP_HealthBar.AttachedCreature` _asbp_enemy _aswbp_health_bar)
  (`/Game/Blueprints/Enemy/WBP_HealthBar.InitHealthBar` _aswbp_health_bar))

(event `self.VisibilityRange.OnComponentBeginOverlap`
  (params (OverlappedComponent :type "PrimitiveComponent Object Reference") (OtherActor :type "Actor Object Reference") (OtherComp :type "PrimitiveComponent Object Reference") (OtherBodyIndex :type Integer) (bFromSweep :type Boolean) (SweepResult :type "HitResult Structure (by ref)"))
  (if (`KismetSystemLibrary.DoesImplementInterface` OtherActor "/Game/Blueprints/Interfaces/BPI_Being.BPI_Being_C")
    (`self.Show`)))

(event `self.VisibilityRange.OnComponentEndOverlap`
  (params (OverlappedComponent :type "PrimitiveComponent Object Reference") (OtherActor :type "Actor Object Reference") (OtherComp :type "PrimitiveComponent Object Reference") (OtherBodyIndex :type Integer))
  (if (`KismetSystemLibrary.DoesImplementInterface` OtherActor "/Game/Blueprints/Interfaces/BPI_Being.BPI_Being_C")
    (`self.Hide`)))

(fn `Hide`
  (`SceneComponent.SetHiddenInGame` (`self.DefaultSceneRoot`) true true))

(fn `Show`
  (`SceneComponent.SetHiddenInGame` (`self.DefaultSceneRoot`) false true))

(fn `UserConstructionScript`)