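; Samurai robot enemy character that performs a melee lunge attack, can be knocked up, and is destroyed when its health runs out.
; Attacking damages hitbox-overlapped actors whose moral alignment differs from its own, launches the robot forward, then returns to running after a retriggerable delay.
; Alignment is queried by message through a Yes/No macro.
; Attack, knockup and hurt reactions play placeholder animations directly on the mesh.
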(event `/Game/Blueprints/Interfaces/BPI_MeleeAttacker.PrepareAttack`
  ;[0.05786 0.0415 0.1562] Placeholder Animation
  (`SkeletalMeshComponent.PlayAnimation` (`self.Mesh`) "/Game/Art/SamuraiRobot/AS_SamuraiRobot_AttackCombo.AS_SamuraiRobot_AttackCombo" false))

(event `/Game/Blueprints/Interfaces/BPI_MeleeAttacker.Attack`
  (`self.OnAttack`)
  (`KismetSystemLibrary.RetriggerableDelay` 0.8)
  ;[0.05786 0.0415 0.1562] Placeholder Animation
  (`SkeletalMeshComponent.PlayAnimation` (`self.Mesh`) "/Game/Art/SamuraiRobot/AS_SamuraiRobot_Run.AS_SamuraiRobot_Run" true))

(event `/Game/Blueprints/Interfaces/BPI_Being.ReceiveKnockup`
  (params (LaunchVelocity :type "Vector Structure"))
  (`self.LaunchCharacter` LaunchVelocity false true)
  ;[0.05786 0.0415 0.1562] Placeholder Animation
  (`KismetSystemLibrary.Delay` 0.01)
  (`SkeletalMeshComponent.PlayAnimation` (`self.Mesh`) "/Game/Art/SamuraiRobot/AS_SamuraiRobot_KnockupLoop.AS_SamuraiRobot_KnockupLoop" false))

(event `self.ReceiveAnyDamage`
  (params (Damage :type "Float (single-precision)") (DamageType :type "DamageType Object Reference") (InstigatedBy :type "Controller Object Reference") (DamageCauser :type "Actor Object Reference"))
  ;[0.05786 0.0415 0.1562] Placeholder Animation (Requires Override for it to work)
  (`self.LoseHealth` Damage)
  (`SkeletalMeshComponent.PlayAnimation` (`self.Mesh`) "/Game/Art/SamuraiRobot/AS_SamuraiRobot_Hurt.AS_SamuraiRobot_Hurt" false)
  (if (<= (`self.HealthPoints`) 0.0)
    (`self.K2_DestroyActor`)))

(fn `GetMoralAlignment`
  (returns (Alignment :type "/Game/Blueprints/Enumerations/EMoralAlignment Enum"))
  (return "NewEnumerator2"))

(fn `OnAttack`
  (locals (HitboxOverlappedActors :type "Array of Actor Object Reference") (AttackLaunchVelocity :type "Float (double-precision)" :default 2000.0))
  (bind _output_get (set `local.HitboxOverlappedActors` (`PrimitiveComponent.GetOverlappingActors` (`self.AttackHitbox`) null)))
  (for _array_element _output_get
    (bind _alignment (message `/Game/Blueprints/Interfaces/BPI_Being.GetMoralAlignment` _array_element))
    (if (`|EnumInequality` _alignment "NewEnumerator2")
      (`GameplayStatics.ApplyDamage` _array_element 1.0 null self)))
  (`self.LaunchCharacter` (* (`self.GetActorForwardVector`) (`local.AttackLaunchVelocity`)) false true))

(fn `UserConstructionScript`
  (`parent.UserConstructionScript`))