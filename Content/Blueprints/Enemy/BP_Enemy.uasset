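; BP_Enemy is an enemy actor that takes damage, shows its health on a bar and is destroyed at zero health.
; Any damage lowers HealthPoints, spawns an explosion at the actor and fires OnHealthChanged.
; That event refreshes the progress bar cached from its WBP_HealthBar widget at BeginPlay.
; Knockup switches the capsule to physics simulation, launches it with a velocity-change impulse and applies damage.
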(event EventBeginPlay
  (|InitializeHealthBar))

(event Game|Damage|EventAnyDamage
  (params (Damage :type Float%20%28single-precision%29) (DamageType :type Damage%20Type%20Object%20Reference) (InstigatedBy :type Controller%20Object%20Reference) (DamageCauser :type Actor%20Object%20Reference))
  (CallFunction|LoseHealth Damage)
  (Effects|SpawnEmitteratLocation "/Game/StarterContent/Particles/P_Explosion.P_Explosion" (Transformation|GetActorLocation))
  (if (<= (Variables|Default|GetHealthPoints) 0.0)
    (Actor|DestroyActor)))

(fn ConstructionScript)

(fn UpdateHealthBar
  (Progress|SetPercent (Variables|Default|GetHealthProgressBar) (|({4FE282FF-4B7F-5A21-7BDE-C3959BF625AB}/{4C63DB65-47EB-59F1-1169-B3979CF2DC2D}))))

(fn Knockup
  (params (NewVelocity :type Vector :default "0, 0, 0") (Damage :type Float%20%28single-precision%29))
  (Physics|SetSimulatePhysics (Variables|Default|GetCapsuleComponent) true)
  (Physics|AddImpulse (Variables|Default|GetCapsuleComponent) NewVelocity "None" true)
  (Game|Damage|ApplyDamage 0 Damage 0 0)
  (return false))

(fn GetMainStageComponent
  (return 0))

(fn LoseHealth
  (params (Damage :type Float%20%28single-precision%29))
  (bind _returnvalue (|({4FE282FF-4B7F-5A21-7BDE-C3959BF625AB}-Damage) Damage))
  (bind _output_get (LocalVariables|SetPreviousHealthPoints (Variables|Default|GetHealthPoints)))
  (Variables|Default|SetHealthPoints _returnvalue)
  (Default|CallOnHealthChanged _output_get _returnvalue))

(event Custom|OnHealthChanged_Event
  (params (PreviousValue :type Float%20%28single-precision%29) (NewValue :type Float%20%28single-precision%29))
  (CallFunction|UpdateHealthBar))