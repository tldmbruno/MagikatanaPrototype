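; BPFL_AlignmentFunctions is a Blueprint function library for sorting actors by moral alignment.
; Its one function, FilterActorsByMoralAlignment, queries each actor in an array with the GetMoralAlignment interface message.
; Actors that match the alignment to exclude go into an excluded array and all others into an included array, and both are returned.
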(fn `Filter Actors by Moral Alignment`
  (params (Actors :type "Array of Actor Object Reference") (AlignmentToExclude :type "/Game/Blueprints/Enumerations/EMoralAlignment Enum" :default "NewEnumerator0"))
  (returns (IncludedActors :type "Array of Actor Object Reference") (ExcludedActors :type "Array of Actor Object Reference"))
  (locals (LocalIncludedActors :type "Array of Actor Object Reference") (LocalExcludedActors :type "Array of Actor Object Reference"))
  (for _array_element Actors
    (bind _alignment (message `/Game/Blueprints/Being/BPI_Being.GetMoralAlignment` _array_element))
    (if (`|EnumEquality` _alignment AlignmentToExclude)
      (`KismetArrayLibrary.Array_Add` (`local.LocalExcludedActors`) _array_element)
      (else
        (`KismetArrayLibrary.Array_Add` (`local.LocalIncludedActors`) _array_element))))
  (return (`local.LocalIncludedActors`) (`local.LocalExcludedActors`)))