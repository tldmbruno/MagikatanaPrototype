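; Homing missile for the Heliturret that chases a target actor and explodes on hit with effects and radial damage.
; Each tick it moves by a swept SetActorLocation using CharacterMovement velocity, eases its rotation toward the target and re-aims that velocity along its forward vector.
; Parent damage handling feeds HealthPoints; at zero it explodes, unless slashing damage killed it, in which case it splits into two sideways-launched fragments without exploding.
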(event `self.ReceiveBeginPlay`
  (if (`KismetSystemLibrary.IsValid` (`self.HomingTargetActor`))
    (`self.SetVelocityToLookDirection` (`self.HomingSpeed`))))

(event `self.ReceiveTick`
  (params (DeltaSeconds :type "Float (single-precision)"))
  (`self.K2_SetActorLocation` (+ (* (`MovementComponent.Velocity` (`self.CharacterMovement`)) DeltaSeconds) (`self.K2_GetActorLocation`)) true)
  (if (and (`KismetSystemLibrary.IsValid` (`self.HomingTargetActor`)) (`KismetSystemLibrary.IsValid` self))
    (`self.LerpLookAtTargetActor` 0.1)
    (`self.SetVelocityToLookDirection` (`self.HomingSpeed`))))

(event `self.ReceiveHit`
  (params (MyComp :type "PrimitiveComponent Object Reference") (Other :type "Actor Object Reference") (OtherComp :type "PrimitiveComponent Object Reference") (bSelfMoved :type Boolean) (HitLocation :type "Vector Structure") (HitNormal :type "Vector Structure") (NormalImpulse :type "Vector Structure") (Hit :type "HitResult Structure (by ref)"))
  (`self.ExplodeSelf` HitLocation))

(event `self.ReceiveAnyDamage`
  (params (Damage :type "Float (single-precision)") (DamageType :type "DamageType Object Reference") (InstigatedBy :type "Controller Object Reference") (DamageCauser :type "Actor Object Reference"))
  (`parent.ReceiveAnyDamage` Damage DamageType InstigatedBy DamageCauser)
  (if (<= (`self.HealthPoints`) 0.0)
    (if (!= (`GameplayStatics.GetObjectClass` DamageType) "/Game/Blueprints/Interfaces/BPI_SlashingDamage.BPI_SlashingDamage_C")
      (`self.ExplodeSelf` (`self.K2_GetActorLocation`))
      (else
        (`self.SpawnDislocatedMissile` 2000.0 50.0)
        (`self.SpawnDislocatedMissile` -2000.0 -50.0)
        (`self.K2_DestroyActor`)))))

(fn `ExplodeSelf`
  (params (ImpactLocation :type "Vector Structure"))
  (`GameplayStatics.SpawnEmitterAtLocation` "/Game/StarterContent/Particles/P_Explosion.P_Explosion" ImpactLocation)
  (`GameplayStatics.SpawnSoundAtLocation` "/Game/StarterContent/Audio/Explosion_Cue.Explosion_Cue" ImpactLocation (struct) 1.0 1.0 0.0 null null)
  (`GameplayStatics.ApplyRadialDamage` :`BaseDamage` (`self.ExplosionDamage`) :`Origin` (`self.K2_GetActorLocation`) :`DamageRadius` (`self.ExplosionDamageRadius`) :`DamageCauser` self :`InstigatedByController` null :`bDoFullDamage` true)
  (`self.K2_DestroyActor`))

(fn `GetMoralAlignment`
  (returns (Alignment :type "/Game/Blueprints/Enumerations/EMoralAlignment Enum"))
  (return "NewEnumerator2"))

(fn `LerpLookAtTargetActor`
  (params (LerpAlpha :type "Float (double-precision)" :default 0.5))
  (`self.K2_SetActorRotation` (`KismetMathLibrary.RLerp` (`self.K2_GetActorRotation`) (`KismetMathLibrary.FindLookAtRotation` (`self.K2_GetActorLocation`) (`self.K2_GetActorLocation` (`self.HomingTargetActor`))) LerpAlpha true)))

(fn `SetVelocityToLookDirection`
  (params (`Homing Speed` :type "Float (double-precision)"))
  (set `MovementComponent.Velocity` (* (`self.GetActorForwardVector`) `Homing Speed`) (`self.CharacterMovement`)))

(fn `SpawnDislocatedMissile`
  (params (RightImpulse :type "Float (double-precision)") (RightOffset :type "Float (double-precision)"))
  (bind (_returnvalue_x _returnvalue_y) (`KismetMathLibrary.BreakVector` (`self.GetVelocity`)))
  (bind (_returnvalue_location _returnvalue_rotation _returnvalue_scale) (`KismetMathLibrary.BreakTransform` (`self.GetTransform`)))
  (bind _returnvalue (`self.GetActorRightVector`))
  (bind _returnvalue_2 (`|SpawnActorFromClass` "/Game/Blueprints/Heliturret/HomingMissile/BP_HomingMissileFragment.BP_HomingMissileFragment_C" (`KismetMathLibrary.MakeTransform` (+ (* _returnvalue RightOffset) _returnvalue_location) _returnvalue_rotation _returnvalue_scale) "Undefined" "OverrideRootScale" null null))
  (`PrimitiveComponent.AddImpulse` (`/Game/Blueprints/Heliturret/HomingMissile/BP_HomingMissileFragment.SphereCollision` _returnvalue_2) (+ (* (`KismetMathLibrary.MakeVector` _returnvalue_x _returnvalue_y) 2.0) (* _returnvalue RightImpulse)) "None" true))

(fn `UserConstructionScript`
  (`parent.UserConstructionScript`))