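; BP_HomingMissileFragment is a heliturret homing missile fragment that explodes when it hits something.
; A hit on its sphere collision calls ExplodeSelf at the actor's location.
; ExplodeSelf spawns an explosion emitter and sound, applies full radial damage without falloff using its damage and radius variables, then destroys the actor.
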(event `self.SphereCollision.OnComponentHit`
  (params (HitComponent :type "PrimitiveComponent Object Reference") (OtherActor :type "Actor Object Reference") (OtherComp :type "PrimitiveComponent Object Reference") (NormalImpulse :type "Vector Structure") (Hit :type "HitResult Structure (by ref)"))
  (`self.ExplodeSelf` (`self.K2_GetActorLocation`)))

(fn `ExplodeSelf`
  (params (Location :type "Vector Structure"))
  (locals (ExplosionDamage :type "Float (double-precision)" :default 1.0) (ExplosionDamageRadius :type "Float (double-precision)" :default 150.0))
  (`GameplayStatics.SpawnEmitterAtLocation` "/Game/UnrealStarterContent/Particles/P_Explosion.P_Explosion" Location)
  (`GameplayStatics.SpawnSoundAtLocation` "/Game/UnrealStarterContent/Audio/Explosion_Cue.Explosion_Cue" Location (struct) 1.0 1.0 0.0 null null)
  (`GameplayStatics.ApplyRadialDamage` :`BaseDamage` (`local.ExplosionDamage`) :`Origin` (`self.K2_GetActorLocation`) :`DamageRadius` (`local.ExplosionDamageRadius`) :`DamageCauser` self :`InstigatedByController` null :`bDoFullDamage` true)
  (`self.K2_DestroyActor`))

(fn `UserConstructionScript`)