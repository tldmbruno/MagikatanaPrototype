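; Heliturret is a flying turret character that fires hitscan shots from its muzzle and forces itself back into Flying whenever its movement mode changes.
; Each attack spends ammo, plays muzzle effects, traces to the target location, draws a bullet line and applies bullet damage.
; The trace uses the Camera channel so cover blocks shots.
; It also exposes ammo reload, ammo count and moral alignment.
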(event `self.K2_OnMovementModeChanged`
  (params (PrevMovementMode :type "EMovementMode Enum" :default "MOVE_None") (NewMovementMode :type "EMovementMode Enum" :default "MOVE_None") (PrevCustomMode :type Byte) (NewCustomMode :type Byte))
  (`CharacterMovementComponent.SetMovementMode` (`self.CharacterMovement`) "MOVE_Flying" 0) ; Keep the engines going
)

(event `self.ReloadAmmo`
  (params (Amount :type Integer))
  (if (!= Amount 0)
    (set `self.Ammo` (`KismetMathLibrary.Clamp` (+ Amount (`self.Ammo`)) 0 (`self.MaxAmmo`)))
    (else
      (set `self.Ammo` (`self.MaxAmmo`)))))

(event `self.PerformRangedAttack`
  (params (HitscanTargetLocation :type "Vector Structure"))
  (bind (_returnvalue_location _returnvalue_rotation) (`KismetMathLibrary.BreakTransform` (`SceneComponent.K2_GetComponentToWorld` (`self.Muzzle`))))
  (bind _returnvalue (`SceneComponent.K2_GetComponentLocation` (`self.Muzzle`)))
  (`/Engine/EditorBlueprintResources/StandardMacros.DecrementInt` (`self.Ammo`)
    (:`  `
      (bind _returnvalue_2 (`NiagaraFunctionLibrary.SpawnSystemAtLocation` "/Game/Art/AttackParticles/NS_CircleImpact.NS_CircleImpact" _returnvalue_location _returnvalue_rotation (1.0 1.0 1.0) true true "AutoRelease"))
      (`FXSystemComponent.SetFloatParameter` _returnvalue_2 "ImpactScale" 0.6)
      (`GameplayStatics.SpawnSoundAtLocation` "/Game/Audio/A_HeavyHitShort.A_HeavyHitShort" _returnvalue_location (struct) 1.0 3.0 0.0 null null)
      (bind _hitresult (`self.ActivateHitscan` _returnvalue HitscanTargetLocation))
      (bind _returnvalue_3 (`NiagaraFunctionLibrary.SpawnSystemAtLocation` "/Game/Art/AttackParticles/NS_BulletLine.NS_BulletLine" _returnvalue))
      (bind (_bblockinghit _binitialoverlap _time _distance _location _impactpoint _normal _impactnormal _physmat _hitactor) (`GameplayStatics.BreakHitResult` _hitresult))
      (`FXSystemComponent.SetVectorParameter` _returnvalue_3 "BulletEndLocation" _impactpoint)
      (`GameplayStatics.ApplyDamage` _hitactor 1.0 (`self.GetController`) self "/Game/Blueprints/Interfaces/BPI_BulletDamage.BPI_BulletDamage_C"))))

(fn `ActivateHitscan`
  (params (MuzzleLocation :type "Vector Structure") (TraceEndLocation :type "Vector Structure"))
  (returns (HitResult :type "HitResult Structure"))
  (locals (ActorsToIgnore :type "Array of Actor Object Reference"))
  (`KismetArrayLibrary.Array_AddUnique` (`local.ActorsToIgnore`) self)
  (bind _outhit (`KismetSystemLibrary.LineTraceSingle` MuzzleLocation TraceEndLocation "TraceTypeQuery2" true (`local.ActorsToIgnore`) "None" true (struct :`R` 1.0 :`G` 0.493973 :`A` 1.0) (struct :`R` 0.527402 :`G` 0.134413 :`B` 1.0 :`A` 1.0) 1.0)) ; It's a Camera TraceChannel to allow the target to hide\nbehind cover, such as walls, pillars or other actors.
  (return _outhit))

(fn `GetAmmoCount`
  (returns (RemainingAmmo :type Integer))
  (return (`self.Ammo`)))

(fn `GetMoralAlignment`
  (returns (Alignment :type "/Game/Blueprints/Enumerations/EMoralAlignment Enum"))
  (return "NewEnumerator2"))

(fn `UserConstructionScript`
  (`parent.UserConstructionScript`)
  (`KismetArrayLibrary.Array_AddUnique` (`self.ActorUnlitMeshes`) (`self.StaticMesh`)))