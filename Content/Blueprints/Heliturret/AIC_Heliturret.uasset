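; AI controller for the Heliturret that runs its behavior tree and picks an attack target from perceived actors.
; Perception updates lock onto a Good or Neutral aligned actor only while no valid target exists, mirroring it to the Blackboard.
; A looping timer works around missing forgotten-stimulus events, switching to the nearest sight-perceived actor, without an alignment check, when the target is invalid or forgotten.
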(event `self.ReceiveBeginPlay`
  (`self.RunBehaviorTree` "/Game/Blueprints/Heliturret/BT_Heliturret.BT_Heliturret")
  (`KismetSystemLibrary.K2_SetTimerDelegate` (`|CreateDelegate` :!event `CheckForForgottenStimuli`) 1.0 true) ; Check periodically if the AI forgot\nany stimuli, since Unreal doesn't have\na proper Event for this.
)

(event `self.AIPerception.OnTargetPerceptionUpdated`
  (params (Actor :type "Actor Object Reference") (Stimulus :type "AIStimulus Structure"))
  (if (not (`KismetSystemLibrary.IsValid` (`self.AttackTargetActor`)))
    (bind _alignment (message `/Game/Blueprints/Interfaces/BPI_Being.GetMoralAlignment` Actor))
    (switch `/Game/Blueprints/Enumerations/EMoralAlignment` _alignment
      (:`NewEnumerator0`
        _)
      (:`NewEnumerator1`
        _))
    (set `self.AttackTargetActor` Actor)
    (`BlackboardComponent.SetValueAsObject` (`self.Blackboard`) (`self.AttackTargetActorName`) Actor)))

(event `CheckForForgottenStimuli`
  (if (`KismetSystemLibrary.IsValid` (`self.AttackTargetActor`))
    (if (not (`KismetArrayLibrary.Array_Contains` (`AIPerceptionComponent.GetKnownPerceivedActors` (`self.AIPerception`) "/Script/AIModule.AISense_Sight") (`self.AttackTargetActor`)))
      (`self.TargetNearestKnownPerceivedActor`))
    (else
      (`self.TargetNearestKnownPerceivedActor`))))

(fn `TargetNearestKnownPerceivedActor`
  (bind (_distance _returnvalue) (`GameplayStatics.FindNearestActor` (`self.K2_GetActorLocation`) (`AIPerceptionComponent.GetKnownPerceivedActors` (`self.AIPerception`) "/Script/AIModule.AISense_Sight")))
  (`BlackboardComponent.SetValueAsObject` (`self.Blackboard`) (`self.AttackTargetActorName`) _returnvalue)
  (set `self.AttackTargetActor` _returnvalue))

(fn `UserConstructionScript`)