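; Interactable actor Blueprint that shows a visual highlight when selected.
; OnSelected and OnUnselected loop over ActorUnlitMeshes and toggle the EnableSelectedVFX scalar parameter on each mesh component's materials.
; The effect itself lives in the materials, while BeginPlay and the construction script only call their parent versions.
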(event `self.ReceiveBeginPlay`
  (`parent.ReceiveBeginPlay`))

(event `/Game/Blueprints/Interfaces/BPI_Interactable.OnSelected`
  (for _array_element (`self.ActorUnlitMeshes`)
    (bind _asmesh_component (cast `MeshComponent` _array_element))
    (`MeshComponent.SetScalarParameterValueOnMaterials` _asmesh_component "EnableSelectedVFX" 1.0)))

(event `/Game/Blueprints/Interfaces/BPI_Interactable.OnUnselected`
  (for _array_element (`self.ActorUnlitMeshes`)
    (bind _asmesh_component (cast `MeshComponent` _array_element))
    (`MeshComponent.SetScalarParameterValueOnMaterials` _asmesh_component "EnableSelectedVFX" 0.0)))

(fn `UserConstructionScript`
  (`parent.UserConstructionScript`))